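; BP_Platform is an overworld moving platform that travels back and forth endlessly between its placed position and an end location.
; On BeginPlay it feeds a float curve into MovementTimeline and converts the relative end location into an adjusted one.
; The timeline lerps the actor's location without sweep.
; When it finishes, it swaps start and end and replays from the start, forming a ping-pong loop.
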(event `self.ReceiveBeginPlay`
  (`TimelineComponent.SetFloatCurve` (`self.Movement Timeline`) (`self.Float Curve`) "Value")
  (`self.Initialize Locations`)
  (`self.Play Timeline`))

(event `Play Timeline`
  (bind (_direction _value) (`Timeline|Movement Timeline` :!via `PlayFromStart`)
    (:`Update`
      (`self.K2_SetActorLocation` (`KismetMathLibrary.VLerp` (`self.Start Location`) (`self.End Location`) _value)))
    (:`Finished`
      (bind (_start _end) (`self.Swap Locations` (`self.Start Location`) (`self.End Location`)))
      (set `self.Start Location` _start)
      (set `self.End Location` _end)
      (`self.Play Timeline`))))

(fn `Swap Locations`
  (params (`Start Initial` :type "Vector Structure") (`End Initial` :type "Vector Structure"))
  (returns (Start :type "Vector Structure") (End :type "Vector Structure"))
  (return `End Initial` `Start Initial`))

(fn `UserConstructionScript`)