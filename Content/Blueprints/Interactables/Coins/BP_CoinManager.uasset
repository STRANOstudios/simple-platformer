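; BP_CoinManager tracks the player's coin score and shows it on screen.
; On BeginPlay it creates a UW_ScoreCanvas widget and binds to the OnCoinTaken event of every BP_Coin already in the level.
; When a coin is taken, it adds the coin's value to TotalScore, disables the coin and pushes the new total to the widget.
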(event `self.ReceiveBeginPlay`
  (bind _returnvalue (`|CreateWidget` "/Game/Blueprints/Interactables/Coins/UW_ScoreCanvas.UW_ScoreCanvas_C"))
  (bind _output_get (set `self.Score UI` _returnvalue))
  (`UserWidget.AddToViewport` _output_get 0)
  (bind _outactors (`GameplayStatics.GetAllActorsOfClass` "/Game/Blueprints/Interactables/Coins/BP_Coin.BP_Coin_C"))
  (bind _output_get_2 (set `self.Coins` _outactors))
  (for _array_element _output_get_2
    (add `/Game/Blueprints/Interactables/Coins/BP_Coin.OnCoinTaken` _array_element (delegate `On Coin Taken`))))

(event `On Coin Taken`
  (params (Coin :type "/Game/Blueprints/Interactables/Coins/BP_Coin Object Reference"))
  (bind _output_get (set `self.Total Score` (+ (`self.Total Score`) (`/Game/Blueprints/Interactables/Coins/BP_Coin.Value` Coin))))
  (`/Game/Blueprints/Interactables/Coins/BP_Coin.Disable Actor` Coin)
  (`/Game/Blueprints/Interactables/Coins/UW_ScoreCanvas.Update Score` (`self.Score UI`) _output_get))

(fn `UserConstructionScript`)